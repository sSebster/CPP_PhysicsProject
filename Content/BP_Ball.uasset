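; Ball Blueprint with a mesh and camera, controlled through an Enhanced Input camera movement action.
; BeginPlay stores references to the mesh and camera.
; The input action feeds controller yaw directly from X and controller pitch from a transformed Y.
; Overlap, Tick and hit events are empty, and earlier actor and spring arm rotation attempts remain disconnected.
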(event OnComponentHit(Mesh)
  (params (HitComponent :type Primitive%20Component%20Object%20Reference) (OtherActor :type Actor%20Object%20Reference) (OtherComp :type Primitive%20Component%20Object%20Reference) (NormalImpulse :type Vector :default "0, 0, 0") (Hit :type Hit%20Result%20Structure%20%28by%20ref%29)))

(event Input|EnhancedActionEvents|EnhancedInputActionIA_CameraMouvement
  (params (ActionValue :type Vector%202D%20Structure) (ElapsedSeconds :type Float%20%28double-precision%29) (TriggeredSeconds :type Float%20%28double-precision%29) (InputAction :type Input%20Action%20Object%20Reference :default "/Game/Input/IA_CameraMouvement.IA_CameraMouvement"))
  (Pawn|Input|AddControllerYawInput (.x ActionValue))
  (bind _result (Math|Float|NegateFloat (.y ActionValue))
    (:%20%20
      (Pawn|Input|AddControllerPitchInput _result))))

(event EventBeginPlay
  (Variables|Default|SetMesh (Variables|Character|GetMesh))
  (Variables|Default|SetBallCamera (Variables|Components|GetCamera)))

(event Collision|EventActorBeginOverlap
  (params (OtherActor :type Actor%20Object%20Reference)))

(event EventTick
  (params (DeltaSeconds :type Float%20%28single-precision%29)))

(fn ConstructionScript)